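; BP_DoorWindow is a sliding door or window actor that opens along world X by MaxAperture when overlapped.
; BeginPlay caches the endpoints, then Timeline_0 lerps the actor open and its update chain calls CloseDoor after a delay.
; CloseDoor runs Timeline_1 to lerp it back.
; IsActive gates setup, opening and closing; ending the overlap clears it, so a pending close is skipped.
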(event `self.ReceiveBeginPlay`
  (if (`self.IsActive`)
    (set `self.VectorStart` (`self.K2_GetActorLocation`))
    (set `self.VectorEnd` (`KismetMathLibrary.MakeVector` (`self.MaxAperture`)))))

(event `self.ReceiveActorBeginOverlap`
  (params (OtherActor :type "Actor Object Reference"))
  (bind _vectorstart (`self.VectorStart`))
  (if (`self.IsActive`)
    (bind (_direction _alpha) (`Timeline|Timeline_0` :!via `PlayFromStart`)
      (:`Update`
        (`self.K2_SetActorLocation` (`KismetMathLibrary.VLerp` _vectorstart (+ _vectorstart (`self.VectorEnd`)) _alpha))
        (`self.K2_SetActorLocation` (`self.K2_GetActorLocation`))
        (`KismetSystemLibrary.Delay` 3.0)
        (`self.CloseDoor`)))))

(event `self.ReceiveActorEndOverlap`
  (params (OtherActor :type "Actor Object Reference"))
  (set `self.isActive` false))

(event `CloseDoor`
  (bind _vectorstart (`self.VectorStart`))
  (if (`self.IsActive`)
    (bind (_direction _alphacerrar) (`Timeline|Timeline_1` :!via `PlayFromStart`)
      (:`Update`
        (`self.K2_SetActorLocation` (`KismetMathLibrary.VLerp` (+ _vectorstart (`self.VectorEnd`)) _vectorstart _alphacerrar))
        (set `self.isActive` true)))))

(fn `UserConstructionScript`)