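; BP_Door is a hinged door actor that swings open when an actor overlaps it and closes when the overlap ends.
; BeginPlay zeroes MainPivot's yaw and negates MaxAngle as the swing target, with all motion gated by IsActive.
; Separate open and close timelines lerp that yaw, and the open timeline stores its final yaw back into the target.
; Begin overlap also prints a debug string, even when inactive.
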(event `self.ReceiveBeginPlay`
  ;[1 1 1] Set rotation begin play
  (if (`self.IsActive`)
    (`SceneComponent.K2_SetRelativeRotation` :`self` (`self.MainPivot`))
    (set `self.privateMaxAngle` (* (`self.MaxAngle`) -1.0))))

(event `self.ReceiveActorBeginOverlap`
  (params (OtherActor :type "Actor Object Reference"))
  (bind _mainpivot (`self.MainPivot`))
  ;[1 1 1] Open the door
  (`KismetSystemLibrary.PrintString` "tocando")
  (if (`self.IsActive`)
    (bind (_direction _newtrack_3) (`Timeline|Timeline_0` :!via `PlayFromStart`)
      (:`Update`
        (`SceneComponent.K2_SetRelativeRotation` _mainpivot (`KismetMathLibrary.MakeRotator` 0.0 0.0 (`KismetMathLibrary.Lerp` 0.0 (`self.privateMaxAngle`) _newtrack_3)) false false))
      (:`Finished`
        (set `self.privateMaxAngle` (.yaw (`SceneComponent.RelativeRotation` _mainpivot)))))))

(event `self.ReceiveActorEndOverlap`
  (params (OtherActor :type "Actor Object Reference"))
  ;[1 1 1] Close the door
  (if (`self.IsActive`)
    (bind (_direction _newtrack_3) (`Timeline|Timeline_1` :!via `PlayFromStart`)
      (:`Update`
        (`SceneComponent.K2_SetRelativeRotation` (`self.MainPivot`) (`KismetMathLibrary.MakeRotator` 0.0 0.0 (`KismetMathLibrary.Lerp` (`self.privateMaxAngle`) 0.0 _newtrack_3)) false false)))))

(fn `UserConstructionScript`)